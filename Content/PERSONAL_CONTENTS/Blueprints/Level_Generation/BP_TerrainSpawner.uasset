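; BP_TerrainSpawner builds endless terrain in chunks of rows laid out along world X.
; On BeginPlay it spawns 31 evenly spaced rows: grass at the start and at row 10, weighted random terrain types elsewhere.
; Row 10 also gets an overlap trigger that, on first contact with BP_Character, spawns another BP_TerrainSpawner just past this chunk, continuing the chain.
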(event `self.ReceiveBeginPlay`
  (bind _spawnlocation (`self.SpawnLocation`))
  (bind _spawnlocation_2 (`self.SpawnLocation`))
  (bind (_returnvalue_x _returnvalue_y _returnvalue_z) (`KismetMathLibrary.BreakVector` (`SceneComponent.K2_GetComponentLocation` (`self.SpawnerMesh`))))
  (for _index (range 31)
    (set `self.SpawnLocation` (`KismetMathLibrary.MakeVector` (+ (* _index (`self.SpawnDistanceMultiplier`)) _returnvalue_x) _returnvalue_y _returnvalue_z))
    (if (`KismetMathLibrary.InRange_IntInt` _index 0 2)
      (`|SpawnActorFromClass` "/Game/PERSONAL_CONTENTS/Blueprints/Terrains/BP_Terrain_Grass.BP_Terrain_Grass_C" (`KismetMathLibrary.MakeTransform` (`self.SpawnLocation`)) "Undefined" "MultiplyWithRoot" null null)
      (elif (`KismetMathLibrary.InRange_IntInt` _index 3 9)
        (switch `int` (`KismetMathLibrary.RandomIntegerInRange` 0 8) :!label _label
          (:`0`
            (`|SpawnActorFromClass` "/Game/PERSONAL_CONTENTS/Blueprints/Terrains/BP_Terrain_Grass.BP_Terrain_Grass_C" (`KismetMathLibrary.MakeTransform` _spawnlocation_2) "Undefined" "MultiplyWithRoot" null null :!label _label_2))
          (:`1`
            (goto _label_2))
          (:`2`
            (goto _label_2))
          (:`3`
            (`|SpawnActorFromClass` "/Game/PERSONAL_CONTENTS/Blueprints/Terrains/BP_Terrain_Road.BP_Terrain_Road_C" (`KismetMathLibrary.MakeTransform` _spawnlocation_2) "Undefined" "MultiplyWithRoot" null null :!label _label_3))
          (:`4`
            (goto _label_3))
          (:`5`
            (`|SpawnActorFromClass` "/Game/PERSONAL_CONTENTS/Blueprints/Terrains/BP_Terrain_Water.BP_Terrain_Water_C" (`KismetMathLibrary.MakeTransform` _spawnlocation_2) "Undefined" "MultiplyWithRoot" null null :!label _label_4))
          (:`6`
            (goto _label_4))
          (:`7`
            (`|SpawnActorFromClass` "/Game/PERSONAL_CONTENTS/Blueprints/Terrains/BP_Terrain_Railroad.BP_Terrain_Railroad_C" (`KismetMathLibrary.MakeTransform` _spawnlocation_2) "Undefined" "MultiplyWithRoot" null null))
          (:`8`
            (`|SpawnActorFromClass` "/Game/PERSONAL_CONTENTS/Blueprints/Terrains/BP_TerrainWaterLilies.BP_TerrainWaterLilies_C" (`KismetMathLibrary.MakeTransform` _spawnlocation_2) "Undefined" "MultiplyWithRoot" null null)))
        (elif (== _index 10)
          (`|SpawnActorFromClass` "/Game/PERSONAL_CONTENTS/Blueprints/Terrains/BP_Terrain_Grass.BP_Terrain_Grass_C" (`KismetMathLibrary.MakeTransform` _spawnlocation) "Undefined" "MultiplyWithRoot" null null)
          (bind _returnvalue (`|SpawnActorFromClass` "/Game/PERSONAL_CONTENTS/Blueprints/Level_Generation/BP_TerrainSpawnerTrigger.BP_TerrainSpawnerTrigger_C" (`KismetMathLibrary.MakeTransform` _spawnlocation) "Undefined" "MultiplyWithRoot" null null))
          (add `Actor.OnActorBeginOverlap` _returnvalue (delegate `RespawnTerrainSpawner`))
          (elif (`KismetMathLibrary.InRange_IntInt` _index 10 30)
            (goto _label)))))))

(event `RespawnTerrainSpawner`
  (params (OverlappedActor :type "Actor Object Reference") (OtherActor :type "Actor Object Reference"))
  (bind (_returnvalue_x _returnvalue_y _returnvalue_z) (`KismetMathLibrary.BreakVector` (`SceneComponent.K2_GetComponentLocation` (`self.SpawnerMesh`))))
  (cast `/Game/PERSONAL_CONTENTS/Characters/BP_Character` OtherActor)
  (`/Engine/EditorBlueprintResources/StandardMacros.DoOnce` false
    (:`Completed`
      (bind _output_get (set `self.SpawnLocation` (`KismetMathLibrary.MakeVector` (+ _returnvalue_x (* (`self.SpawnDistanceMultiplier`) 31)) _returnvalue_y _returnvalue_z)))
      (`|SpawnActorFromClass` "BP_TerrainSpawner_C" (`KismetMathLibrary.MakeTransform` _output_get) "Undefined" "MultiplyWithRoot" null null))))

(fn `UserConstructionScript`)