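; Moving road obstacle that kills the player character on overlap.
; Construction script feeds its initial and max speed variables into the projectile movement component, and BeginPlay can swap in one of five alternate meshes based on MeshSelection.
; On overlap with a player-tagged character, the X offset picks a left or right splat socket on the obstacle, or a plain non-splat death when nearly aligned.
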(event `self.ReceiveBeginPlay`
  (bind _objectmesh (`self.ObjectMesh`))
  (switch `int` (`self.MeshSelection`)
    (:`1`
      (`StaticMeshComponent.SetStaticMesh` _objectmesh (`self.AltObjectMesh1`)))
    (:`2`
      (`StaticMeshComponent.SetStaticMesh` _objectmesh (`self.AltObjectMesh2`)))
    (:`3`
      (`StaticMeshComponent.SetStaticMesh` _objectmesh (`self.AltObjectMesh3`)))
    (:`4`
      (`StaticMeshComponent.SetStaticMesh` _objectmesh (`self.AltObjectMesh4`)))
    (:`5`
      (`StaticMeshComponent.SetStaticMesh` _objectmesh (`self.AltObjectMesh5`)))))

(event `self.ReceiveActorBeginOverlap`
  (params (OtherActor :type "Actor Object Reference"))
  (bind _returnvalue_x (`KismetMathLibrary.BreakVector` (`self.K2_GetActorLocation`)))
  (bind _returnvalue_x_2 (`KismetMathLibrary.BreakVector` (`self.K2_GetActorLocation` OtherActor)))
  (bind _returnvalue (- _returnvalue_x_2 _returnvalue_x))
  (if (`self.ActorHasTag` OtherActor "player")
    (bind _asbp_character (cast `/Game/PERSONAL_CONTENTS/Characters/BP_Character` OtherActor))
    (if (> _returnvalue 0.5)
      (`CrossyRoadCharacter.Death` _asbp_character self true "SplatSX")
      (elif (< _returnvalue -0.5)
        (`CrossyRoadCharacter.Death` _asbp_character self true "SplatDX")
        (else
          (`CrossyRoadCharacter.Death` _asbp_character null false "None"))))))

(fn `UserConstructionScript`
  (bind _projectilemovement (`self.ProjectileMovement`))
  (set `ProjectileMovementComponent.InitialSpeed` (`self.ObjectInitialSpeed`) _projectilemovement)
  (set `ProjectileMovementComponent.MaxSpeed` (`self.ObjectMaxSpeed`) _projectilemovement))