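; Police car hazard that moves by projectile movement and kills the player character on overlap.
; The construction script copies the object's initial and max speed variables into the ProjectileMovement component.
; On overlap with a "player"-tagged BP_Character, the X offset picks the death: side hits splat it onto the car's SplatSX or SplatDX socket, while near-centered hits kill without a splat.
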(event `self.ReceiveActorBeginOverlap`
  (params (OtherActor :type "Actor Object Reference"))
  (bind _returnvalue_x (`KismetMathLibrary.BreakVector` (`self.K2_GetActorLocation`)))
  (bind _returnvalue_x_2 (`KismetMathLibrary.BreakVector` (`self.K2_GetActorLocation` OtherActor)))
  (bind _returnvalue (- _returnvalue_x_2 _returnvalue_x))
  (if (`self.ActorHasTag` OtherActor "player")
    (bind _asbp_character (cast `/Game/PERSONAL_CONTENTS/Characters/BP_Character` OtherActor))
    (if (> _returnvalue 0.5)
      (`CrossyRoadCharacter.Death` _asbp_character self true "SplatSX")
      (elif (< _returnvalue -0.5)
        (`CrossyRoadCharacter.Death` _asbp_character self true "SplatDX")
        (else
          (`CrossyRoadCharacter.Death` _asbp_character null false "None"))))))

(fn `UserConstructionScript`
  (bind _projectilemovement (`self.ProjectileMovement`))
  (set `ProjectileMovementComponent.InitialSpeed` (`self.ObjectInitialSpeed`) _projectilemovement)
  (set `ProjectileMovementComponent.MaxSpeed` (`self.ObjectMaxSpeed`) _projectilemovement))