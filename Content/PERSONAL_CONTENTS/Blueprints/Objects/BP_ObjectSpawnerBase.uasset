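; Base Blueprint for a moving object with a projectile movement component and a randomly varied static mesh.
; On BeginPlay it copies its initial and max speed variables into the projectile movement component.
; It then rolls a random integer up to AltMeshes and swaps in the first alternate mesh on a result of 1; other results keep the current mesh.
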(event `self.ReceiveBeginPlay`
  (bind _projectilemovement (`self.ProjectileMovement`))
  (set `ProjectileMovementComponent.InitialSpeed` (`self.ObjectInitialSpeed`) _projectilemovement)
  (set `ProjectileMovementComponent.MaxSpeed` (`self.ObjectMaxSpeed`) _projectilemovement)
  (switch `int` (`KismetMathLibrary.RandomIntegerInRange` 0 (`self.AltMeshes`))
    (:`1`
      (`StaticMeshComponent.SetStaticMesh` (`self.ObjectMesh`) (`self.AltObjectMesh1`)))))

(fn `UserConstructionScript`)