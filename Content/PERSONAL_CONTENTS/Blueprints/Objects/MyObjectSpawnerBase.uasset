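; MyObjectSpawnerBase is a base Blueprint for an object with a mesh and projectile movement, tunable per instance or subclass.
; The construction script copies initial and maximum speed variables into the projectile movement component.
; On BeginPlay, a switch on MeshSelection swaps in an alternate static mesh for selection 1, otherwise leaving the default mesh.
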(event `self.ReceiveBeginPlay`
  (switch `int` (`self.MeshSelection`)
    (:`1`
      (`StaticMeshComponent.SetStaticMesh` (`self.ObjectMesh`) (`self.AltObjectMesh1`)))))

(fn `UserConstructionScript`
  (bind _projectilemovement (`self.ProjectileMovement`))
  (set `ProjectileMovementComponent.InitialSpeed` (`self.ObjectInitialSpeed`) _projectilemovement)
  (set `ProjectileMovementComponent.MaxSpeed` (`self.ObjectMaxSpeed`) _projectilemovement))