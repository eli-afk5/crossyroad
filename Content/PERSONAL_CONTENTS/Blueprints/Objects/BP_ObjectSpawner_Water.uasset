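; BP_ObjectSpawner_Water is an actor that dips and rises when a player-tagged actor overlaps it, like a floating log; no spawning logic is present.
; Overlap runs the MoveLogDown timeline toward 20 units lower, then MoveLogUp toward 20 units higher, lerping from the current location each update.
; Two DoOnce gates block retriggering and reset after the rise finishes.
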(event `self.ReceiveActorBeginOverlap`
  (params (OtherActor :type "Actor Object Reference"))
  (bind (_returnvalue_x _returnvalue_y _returnvalue_z) (`KismetMathLibrary.BreakVector` (`self.K2_GetActorLocation`)))
  (if (`self.ActorHasTag` OtherActor "player")
    (`KismetSystemLibrary.PrintString` "Hello" true true (struct :`R` 1.0 :`G` 0.353516 :`A` 1.0))
    (`/Engine/EditorBlueprintResources/StandardMacros.DoOnce` false :!label _label
      (:`Completed`
        (set `self.NewZ` (- _returnvalue_z 20.0))
        (bind (_direction _alpha) (`Timeline|MoveLogDown` :!via `PlayFromStart`)
          (:`Update`
            (`self.K2_SetActorLocation` (`KismetMathLibrary.VLerp` (`self.K2_GetActorLocation`) (`KismetMathLibrary.MakeVector` _returnvalue_x _returnvalue_y (`self.NewZ`)) _alpha)))
          (:`Finished`
            (`/Engine/EditorBlueprintResources/StandardMacros.DoOnce` false :!label _label_2
              (:`Completed`
                (set `self.NewZ` (+ _returnvalue_z 20.0))
                (bind (_direction_2 _alpha_2) (`Timeline|MoveLogUp` :!via `PlayFromStart`)
                  (:`Update`
                    (`self.K2_SetActorLocation` (`KismetMathLibrary.VLerp` (`self.K2_GetActorLocation`) (`KismetMathLibrary.MakeVector` _returnvalue_x _returnvalue_y (`self.NewZ`)) _alpha_2)))
                  (:`Finished`
                    (`|ExecutionSequence`
                      (:`then_0`
                        (goto _label :!via `Reset`))
                      (:`then_1`
                        (goto _label_2 :!via `Reset`)))))))))))))

(fn `UserConstructionScript`)