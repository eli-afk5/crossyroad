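; BP_RailroadSignal is a railroad signal object with two lights and a signal sound.
; StartSignal swaps each light to its own signal material and plays the sound from the beginning.
; StopLights returns both lights to a shared base material but does not stop the sound.
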(event `StartSignal`
  (`PrimitiveComponent.SetMaterial` (`self.Light1`) 0 "/Game/PERSONAL_CONTENTS/Materials/Placeholders/Objects/MI_ObjectTrainSignal_Light1.MI_ObjectTrainSignal_Light1")
  (`PrimitiveComponent.SetMaterial` (`self.Light2`) 0 "/Game/PERSONAL_CONTENTS/Materials/Placeholders/Objects/MI_ObjectTrainSignal_Light2.MI_ObjectTrainSignal_Light2")
  (`AudioComponent.Play` (`self.SignalSound`) 0.0))

(event `StopLights`
  (`PrimitiveComponent.SetMaterial` (`self.Light1`) 0 "/Game/PERSONAL_CONTENTS/Materials/Placeholders/Objects/MI_ObjectTrainSignal_LightBase.MI_ObjectTrainSignal_LightBase")
  (`PrimitiveComponent.SetMaterial` (`self.Light2`) 0 "/Game/PERSONAL_CONTENTS/Materials/Placeholders/Objects/MI_ObjectTrainSignal_LightBase.MI_ObjectTrainSignal_LightBase"))

(fn `UserConstructionScript`)