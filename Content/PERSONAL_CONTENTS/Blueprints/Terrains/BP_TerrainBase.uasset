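; BP_TerrainBase is a base terrain Blueprint that awards score when the player reaches it.
; On BeginPlay it caches the world locations of its spawner start and end points, which this graph does not use further.
; An overlap by an actor tagged "player" casts to BP_Character and calls IncreaseScore through a DoOnce, so each terrain instance scores only once.
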(event `self.ReceiveBeginPlay`
  (set `self.SpawnerStartLocation` (`SceneComponent.K2_GetComponentLocation` (`self.SpawnerStartPoint`)))
  (set `self.SpawnerEndLocation` (`SceneComponent.K2_GetComponentLocation` (`self.SpawnerEndPoint`))))

(event `self.ReceiveActorBeginOverlap`
  (params (OtherActor :type "Actor Object Reference"))
  (if (`self.ActorHasTag` OtherActor "player")
    (bind _asbp_character (cast `/Game/PERSONAL_CONTENTS/Characters/BP_Character` OtherActor)
      (:`then`
        (`/Engine/EditorBlueprintResources/StandardMacros.DoOnce` false
          (:`Completed`
            (`/Game/PERSONAL_CONTENTS/Characters/BP_Character.IncreaseScore` _asbp_character))))
      (:`CastFailed`
        (`KismetSystemLibrary.PrintString` "Cast Fail")))))

(fn `UserConstructionScript`)