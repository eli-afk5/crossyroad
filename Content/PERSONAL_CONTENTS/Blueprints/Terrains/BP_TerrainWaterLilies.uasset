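; BP_TerrainWaterLilies is a water terrain piece that places water lily spawners and drowns the player.
; On BeginPlay, after the parent logic, it steps along Y from the spawner start location, with a step count derived from the start-to-end distance.
; A random check at each step decides whether a BP_ObjectSpawner_WaterLilies is spawned, leaving irregular gaps.
; Overlapping the BoxDrown volume calls Death on a player-tagged BP_Character.
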(event `self.ReceiveBeginPlay`
  (bind (_spawnerstartlocation_x _spawnerstartlocation_y _spawnerstartlocation_z) (`KismetMathLibrary.BreakVector` (`self.SpawnerStartLocation`)))
  (`parent.ReceiveBeginPlay`)
  (for _index (range (+ (`KismetMathLibrary.FTrunc` (/ (`KismetMathLibrary.Vector_Distance` (`self.SpawnerStartLocation`) (`self.SpawnerEndLocation`)) (`self.StartEndDistanceDivisor`))) 1))
    (if (> (`KismetMathLibrary.RandomFloat`) (`self.SpawnIntervalCondition`))
      (`|SpawnActorFromClass` "/Game/PERSONAL_CONTENTS/Blueprints/Objects/BP_ObjectSpawner_WaterLilies.BP_ObjectSpawner_WaterLilies_C" (`KismetMathLibrary.MakeTransform` (`KismetMathLibrary.MakeVector` _spawnerstartlocation_x (+ (* _index (`self.SpawnIntervalMultiplier`)) _spawnerstartlocation_y) _spawnerstartlocation_z)) "Undefined" "MultiplyWithRoot" null null))))

(event `self.Box Drown.OnComponentBeginOverlap`
  (params (OverlappedComponent :type "PrimitiveComponent Object Reference") (OtherActor :type "Actor Object Reference") (OtherComp :type "PrimitiveComponent Object Reference") (OtherBodyIndex :type Integer) (bFromSweep :type Boolean) (SweepResult :type "HitResult Structure (by ref)"))
  (if (`self.ActorHasTag` OtherActor "player")
    (bind _asbp_character (cast `/Game/PERSONAL_CONTENTS/Characters/BP_Character` OtherActor))
    (`CrossyRoadCharacter.Death` _asbp_character)))

(fn `UserConstructionScript`
  (`parent.UserConstructionScript`))