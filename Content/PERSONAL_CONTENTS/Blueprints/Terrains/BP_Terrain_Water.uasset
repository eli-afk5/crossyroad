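; BP_Terrain_Water is a water lane terrain that spawns moving objects and drowns the player on contact.
; On BeginPlay it randomly picks which end to spawn from and starts a looping timer with an interval randomized once.
; Each tick of that timer spawns a BP_ObjectSpawner_Water at the lane speed, with lifespan inversely proportional to speed.
; Overlapping BoxDrown calls Death without splatting on a player-tagged BP_Character.
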(event `self.ReceiveBeginPlay`
  (`parent.ReceiveBeginPlay`)
  (set `self.bSpawnFromStart` (`KismetMathLibrary.RandomBool`))
  (`KismetSystemLibrary.K2_SetTimerDelegate` (delegate `SpawnProjectileObject`) (`KismetMathLibrary.RandomFloatInRange` (`self.MinSpawnInterval`) (`self.MaxSpawnInterval`)) true))

(event `SpawnProjectileObject`
  (bind _lanespeed (`self.LaneSpeed`))
  (bind _returnvalue (/ 2000.0 (`self.LaneSpeed`)))
  (if (`self.bSpawnFromStart`)
    (bind _returnvalue_2 (`|SpawnActorFromClass` "/Game/PERSONAL_CONTENTS/Blueprints/Objects/BP_ObjectSpawner_Water.BP_ObjectSpawner_Water_C" (`KismetMathLibrary.MakeTransform` (`self.SpawnerStartLocation`) (struct :`Yaw` 90.0)) "Undefined" "MultiplyWithRoot" null _lanespeed _lanespeed null))
    (`self.SetLifeSpan` _returnvalue_2 _returnvalue)
    (else
      (bind _returnvalue_3 (`|SpawnActorFromClass` "/Game/PERSONAL_CONTENTS/Blueprints/Objects/BP_ObjectSpawner_Water.BP_ObjectSpawner_Water_C" (`KismetMathLibrary.MakeTransform` (`self.SpawnerEndLocation`) (struct :`Yaw` -90.0)) "Undefined" "MultiplyWithRoot" null _lanespeed _lanespeed null))
      (`self.SetLifeSpan` _returnvalue_3 _returnvalue))))

(event `self.Box Drown.OnComponentBeginOverlap`
  (params (OverlappedComponent :type "PrimitiveComponent Object Reference") (OtherActor :type "Actor Object Reference") (OtherComp :type "PrimitiveComponent Object Reference") (OtherBodyIndex :type Integer) (bFromSweep :type Boolean) (SweepResult :type "HitResult Structure (by ref)"))
  (if (`self.ActorHasTag` OtherActor "player")
    (bind _asbp_character (cast `/Game/PERSONAL_CONTENTS/Characters/BP_Character` OtherActor))
    (`CrossyRoadCharacter.Death` _asbp_character null false "None")))

(fn `UserConstructionScript`
  (`parent.UserConstructionScript`))