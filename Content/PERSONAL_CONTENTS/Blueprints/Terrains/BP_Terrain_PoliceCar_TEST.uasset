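; Test terrain lane that spawns police car objects, extending a parent Blueprint.
; BeginPlay calls InitializeLane, which stores lane speed, randomly picks a mesh index and spawn side, and starts a looping timer with a once-randomized interval.
; SpawnRoadObject creates BP_ObjectSpawner_PoliceCar at the chosen end, facing the matching direction, with lifespan inversely proportional to lane speed.
; A leftover random gate before spawning is disconnected.
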(event `self.ReceiveBeginPlay`
  (`parent.ReceiveBeginPlay`)
  (`self.InitializeLane` (`self.LaneSpeed`)))

(event `SpawnRoadObject`
  (if (`self.bSpawnFromStart`)
    (bind _returnvalue (`|SpawnActorFromClass` "/Game/PERSONAL_CONTENTS/Blueprints/Objects/BP_ObjectSpawner_PoliceCar.BP_ObjectSpawner_PoliceCar_C" (`KismetMathLibrary.MakeTransform` (`self.SpawnerStartLocation`) (struct :`Yaw` 90.0)) "Undefined" "MultiplyWithRoot" null 2000.0 null))
    (`self.SetLifeSpan` _returnvalue (/ 2000.0 (`self.LaneSpeed`)))
    (else
      (bind _returnvalue_2 (`|SpawnActorFromClass` "/Game/PERSONAL_CONTENTS/Blueprints/Objects/BP_ObjectSpawner_PoliceCar.BP_ObjectSpawner_PoliceCar_C" (`KismetMathLibrary.MakeTransform` (`self.SpawnerEndLocation`) (struct :`Yaw` -90.0)) "Undefined" "MultiplyWithRoot" null 2000.0 null))
      (`self.SetLifeSpan` _returnvalue_2 (/ 2000.0 (`self.LaneSpeed`))))))

(fn `InitializeLane`
  (params (RandomSpeed :type "Float (double-precision)"))
  (set `self.LaneSpeed` RandomSpeed)
  (set `self.LaneMeshSelection` (`KismetMathLibrary.RandomIntegerInRange` 0 (`self.LaneAltMeshes`)))
  (set `self.bSpawnFromStart` (`KismetMathLibrary.RandomBool`))
  (`KismetSystemLibrary.K2_ClearAndInvalidateTimerHandle` (`self.LaneTimerHandle`))
  (bind _returnvalue (`KismetSystemLibrary.K2_SetTimerDelegate` (`|CreateDelegate` :!event `SPawnRoadObject`) (`KismetMathLibrary.RandomFloatInRange` (`self.MinSpawnInterval`) (`self.MaxSpawnInterval`)) true))
  (set `self.LaneTimerHandle` _returnvalue))

(fn `UserConstructionScript`)