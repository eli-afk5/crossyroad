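; BP_TerrainGrass is a grass terrain Blueprint that randomly populates a line with spawned actors when play begins.
; After the parent BeginPlay, it derives a step count from the distance between the spawner start and end locations and a divisor.
; Each step that passes a random threshold check spawns the configured actor class, offset from the start along world Y only by the interval multiplier.
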(event `self.ReceiveBeginPlay`
  (bind (_spawnerstartlocation_x _spawnerstartlocation_y _spawnerstartlocation_z) (`KismetMathLibrary.BreakVector` (`self.SpawnerStartLocation`)))
  (`parent.ReceiveBeginPlay`)
  (for _index (range (+ (`KismetMathLibrary.FTrunc` (/ (`KismetMathLibrary.Vector_Distance` (`self.SpawnerStartLocation`) (`self.SpawnerEndLocation`)) (`self.StartEndDistanceDivisor`))) 1))
    (if (> (`KismetMathLibrary.RandomFloat`) (`self.SpawnIntervalCondition`))
      (`|SpawnActorFromClass` (`self.SpawnedActorClass`) (`KismetMathLibrary.MakeTransform` (`KismetMathLibrary.MakeVector` _spawnerstartlocation_x (+ (* _index (`self.SpawnIntervalMultiplier`)) _spawnerstartlocation_y) _spawnerstartlocation_z)) "Undefined" "MultiplyWithRoot" null null))))

(fn `UserConstructionScript`
  (`parent.UserConstructionScript`))