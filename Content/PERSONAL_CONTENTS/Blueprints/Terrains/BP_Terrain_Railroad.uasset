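; Railroad terrain that periodically sends traffic along its lane from one end, picked at random on BeginPlay.
; A looping timer with a randomised interval spawns a railroad object spawner at that end, passing it the lane speed.
; It also spawns a railroad signal whose light delay comes from a separate random roll of the same range.
; Spawner lifespan and light duration derive from a fixed distance, lane speed and frame delta.
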(event `self.ReceiveBeginPlay`
  (bind _returnvalue (`KismetMathLibrary.RandomFloatInRange` (`self.MinSpawnInterval`) (`self.MaxSpawnInterval`)))
  (`parent.ReceiveBeginPlay`)
  (set `self.bSpawnFromStart` (`KismetMathLibrary.RandomBool`))
  (`KismetSystemLibrary.K2_SetTimerDelegate` (delegate `CustomEvent`) _returnvalue true)
  (`|SpawnActorFromClass` "/Game/PERSONAL_CONTENTS/Blueprints/Objects/BP_RailroadSignal.BP_RailroadSignal_C" (`KismetMathLibrary.MakeTransform` (`SceneComponent.K2_GetComponentLocation` (`self.Signal Spawn Point`)) (struct :`Yaw` 180.0)) "Undefined" "MultiplyWithRoot" null (- _returnvalue 1.0) (+ (/ 2000.0 (* (`self.LaneSpeed`) (`self.DeltaSeconds`))) 1.0) null))

(event `CustomEvent`
  (bind _lanespeed (`self.LaneSpeed`))
  (if (`self.bSpawnFromStart`)
    (bind _returnvalue (`|SpawnActorFromClass` "/Game/PERSONAL_CONTENTS/Blueprints/Objects/BP_ObjectSpawner_Railroad.BP_ObjectSpawner_Railroad_C" (`KismetMathLibrary.MakeTransform` (`self.SpawnerStartLocation`) (struct :`Yaw` 90.0)) "Undefined" "MultiplyWithRoot" null _lanespeed _lanespeed null))
    (`self.SetLifeSpan` _returnvalue (+ (/ 2000.0 (* (`self.LaneSpeed`) (`self.DeltaSeconds`))) 0.25))
    (else
      (bind _returnvalue_2 (`|SpawnActorFromClass` "/Game/PERSONAL_CONTENTS/Blueprints/Objects/BP_ObjectSpawner_Railroad.BP_ObjectSpawner_Railroad_C" (`KismetMathLibrary.MakeTransform` (`self.SpawnerEndLocation`) (struct :`Yaw` -90.0)) "Undefined" "MultiplyWithRoot" null _lanespeed _lanespeed null))
      (`self.SetLifeSpan` _returnvalue_2 (+ (/ 2000.0 (* (`self.LaneSpeed`) (`self.DeltaSeconds`))) 0.25)))))

(event `self.ReceiveTick`
  (params (DeltaSeconds :type "Float (single-precision)"))
  (set `self.DeltaSeconds` DeltaSeconds))

(fn `UserConstructionScript`
  (`parent.UserConstructionScript`))