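; BP_Terrain_Grass is a grass terrain piece that randomly populates itself with grass object spawners when play begins.
; It steps along the Y axis from the spawner start location, with the step count derived from the start-to-end distance.
; At each step, a random roll against a threshold decides whether to spawn a BP_ObjectSpawner_Grass, which receives the lane speed as both initial and maximum object speed.
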(event `self.ReceiveBeginPlay`
  (bind _lanespeed (`self.LaneSpeed`))
  (bind (_spawnerstartlocation_x _spawnerstartlocation_y _spawnerstartlocation_z) (`KismetMathLibrary.BreakVector` (`self.SpawnerStartLocation`)))
  (`parent.ReceiveBeginPlay`)
  (for _index (range (+ (`KismetMathLibrary.FTrunc` (/ (`KismetMathLibrary.Vector_Distance` (`self.SpawnerStartLocation`) (`self.SpawnerEndLocation`)) (`self.StartEndDistanceDivisor`))) 1))
    (if (> (`KismetMathLibrary.RandomFloat`) (`self.SpawnIntervalCondition`))
      (`|SpawnActorFromClass` "/Game/PERSONAL_CONTENTS/Blueprints/Objects/BP_ObjectSpawner_Grass.BP_ObjectSpawner_Grass_C" (`KismetMathLibrary.MakeTransform` (`KismetMathLibrary.MakeVector` _spawnerstartlocation_x (+ (* _index (`self.SpawnIntervalMultiplier`)) _spawnerstartlocation_y) _spawnerstartlocation_z)) "Undefined" "MultiplyWithRoot" null _lanespeed _lanespeed null))))

(fn `UserConstructionScript`
  (`parent.UserConstructionScript`))