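; Player chicken character for a Crossy Road-style hopper, with score, start and lose widgets.
; Held input shows a squish mesh and box-traces for "obstacle" actors, then triggering launches a grid-snapped hop with timeline-driven movement and rotation.
; The camera boom keeps fixed height and creeps forward once first input starts the game.
; IncreaseScore resets that offset, backward hops increase it, and exceeding the limit triggers death, flattening the mesh.
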(event `EnhancedInput|/Game/Input/Actions/IA_Move`
  (params (ActionValue :type "Vector2D Structure") (ElapsedSeconds :type "Float (double-precision)") (TriggeredSeconds :type "Float (double-precision)") (InputAction :type "InputAction Object Reference" :default "/Game/Input/Actions/IA_Move.IA_Move"))
  (bind _returnvalue (`self.K2_GetActorLocation`))
  (bind (_returnvalue_x _returnvalue_y _returnvalue_z) (`KismetMathLibrary.BreakVector` (`self.K2_GetActorLocation`)))
  (bind _sidewaysmovementstrength (`self.SidewaysMovementStrength`))
  (bind _squishmesh (`self.SquishMesh`))
  (bind _defaultmesh (`self.DefaultMesh`))
  (bind _cameraboom (`self.CameraBoom`))
  (bind _defaultmesh_2 (`self.DefaultMesh`))
  (bind _action_value_y (`self.Action Value Y`))
  (bind _action_value_x (`self.Action Value X`))
  (bind (_relativerotation_roll _relativerotation_pitch _relativerotation_yaw) (`KismetMathLibrary.BreakRotator` (`SceneComponent.RelativeRotation` _defaultmesh_2)))
  (:`Triggered`
    ; Move character if they're grounded and there are no obstacles, if alive
    (if (and (and (`NavMovementComponent.IsMovingOnGround` (`self.CharacterMovement`)) (`self.CanMove`)) (not (`self.IsDead`)))
      ; Rounds current location
      (bind _newvalue (`self.RoundMovement` _returnvalue_x))
      (bind _newvalue_2 (`self.RoundMovement` _returnvalue_y))
      (`|ExecutionSequence`
        (:`then_0`
          ; XY movement
          (`/Engine/EditorBlueprintResources/StandardMacros.DoOnce` false :!label _label
            (:`Completed`
              (bind _output_get (set `self.Destination` (`KismetMathLibrary.MakeVector` (+ (* _action_value_y _sidewaysmovementstrength) _newvalue) (+ (* _action_value_x _sidewaysmovementstrength) _newvalue_2) _returnvalue_z)))
              (bind (_direction _movealpha) (`Timeline|SmoothMove` :!via `PlayFromStart`)
                (:`Update`
                  ;; TODO substitute this for an actual squish
                  (`self.K2_SetActorLocation` (`KismetMathLibrary.VLerp` (`self.K2_GetActorLocation`) (`KismetMathLibrary.MakeVector` (.x _output_get) (.y _output_get) _returnvalue_z) _movealpha)))
                (:`Finished`
                  (goto _label :!via `Reset`))))))
        (:`then_1`
          ; Z movement
          (`self.LaunchCharacter` (`KismetMathLibrary.MakeVector` 0.0 0.0 (`self.UpwardMovementStrength`)) false true)
          ; Rotate
          (bind _output_get_2 (set `self.CurrentDirection` (`KismetMathLibrary.DegAtan2` _action_value_x _action_value_y)))
          (bind (_direction_2 _rotationalpha) (`Timeline|Rotate` :!via `PlayFromStart`)
            (:`Update`
              (`SceneComponent.K2_SetRelativeRotation` _defaultmesh_2 (`KismetMathLibrary.RLerp` (`KismetMathLibrary.MakeRotator` _relativerotation_roll _relativerotation_pitch _relativerotation_yaw) (`KismetMathLibrary.MakeRotator` _relativerotation_roll _relativerotation_pitch _output_get_2) _rotationalpha true) false false)
              (`SceneComponent.K2_SetRelativeRotation` (`self.SquishMesh`) (`KismetMathLibrary.RLerp` (`KismetMathLibrary.MakeRotator` _relativerotation_roll _relativerotation_pitch _relativerotation_yaw) (`KismetMathLibrary.MakeRotator` _relativerotation_roll _relativerotation_pitch _output_get_2) _rotationalpha true) false false)
              ; Reset camera offset if moving forward, moves forward if going backward
              (if (< (`self.Action Value Y`) 0.0)
                (set `SpringArmComponent.TargetOffset` (+ (`SpringArmComponent.TargetOffset` _cameraboom) (1.5 0.0 0.0)) _cameraboom))))))))
  (:`Ongoing`
    ; Unpause game if it's the first input
    (if (and (`self.IsGamePaused`) (not (`self.IsDead`)))
      (set `self.IsGamePaused` false)
      (`/Engine/EditorBlueprintResources/StandardMacros.DoOnce` false
        (:`Completed`
          (`/Game/PERSONAL_CONTENTS/Widgets/WB_Start.FadeOut` (stale `self.ReceiveBeginPlay` _returnvalue_3))))
      (else
        ; Set XY movement values
        (bind _output_get_3 (set `self.Action Value X` ActionValue_X))
        (if (> (`KismetMathLibrary.Abs` _output_get_3) 0.0)
          (set `self.Action Value Y` 0.0)
          (else
            (set `self.Action Value Y` ActionValue_Y)))
        (`SceneComponent.SetVisibility` _squishmesh true false)
        (`SceneComponent.SetVisibility` _defaultmesh false false)
        ; Check if there are obstacles in the direction the player wants to move
        (bind (_outhit _returnvalue_2) (`KismetSystemLibrary.BoxTraceSingle` :`Start` _returnvalue :`End` (+ _returnvalue (* (`KismetMathLibrary.MakeVector` (`self.Action Value Y`) (`self.Action Value X`)) 100.0)) :`HalfSize` (10.0 10.0 10.0) :`Orientation` (struct :`Yaw` -90.0) :`TraceChannel` "TraceTypeQuery1" :`DrawDebugType` "ForDuration"))
        (set `self.Out Hit Hit Actor` (`.HitActor` (`GameplayStatics.BreakHitResult` _outhit)))
        (bind _out_hit_hit_actor (`self.Out Hit Hit Actor`)
          (:`then`
            (if (and _returnvalue_2 (`self.ActorHasTag` _out_hit_hit_actor "obstacle"))
              (set `self.CanMove` false)
              (else
                (set `self.CanMove` true :!label _label_2))))
          (:`else`
            (goto _label_2))))))
  (:`Completed`
    (`SceneComponent.SetVisibility` _squishmesh false false)
    (`SceneComponent.SetVisibility` _defaultmesh true false)))

(event `IncreaseScore`
  ; Reset camera offset if moving forward, moves forward if going backward
  (`/Engine/EditorBlueprintResources/StandardMacros.IncrementFloat` (`self.Score`)
    (:`  `
      (set `SpringArmComponent.TargetOffset` (0.0 0.0 0.0) (`self.CameraBoom`)))))

(event `self.ReceiveBeginPlay`
  (bind _returnvalue (`GameplayStatics.GetPlayerController` 0))
  ; Setup score UI
  (bind _returnvalue_2 (`|CreateWidget` "/Game/PERSONAL_CONTENTS/Widgets/WB_ScoreUI.WB_ScoreUI_C" _returnvalue))
  (`UserWidget.AddToViewport` _returnvalue_2 0)
  (set `/Game/PERSONAL_CONTENTS/Widgets/WB_ScoreUI.PlayerRef` self _returnvalue_2)
  ; start screen
  (bind _returnvalue_3 (`|CreateWidget` "/Game/PERSONAL_CONTENTS/Widgets/WB_Start.WB_Start_C" _returnvalue))
  (`UserWidget.AddToViewport` _returnvalue_3 0)
  ; Don't start game until first input
  (set `self.IsGamePaused` true))

(event `self.ReceiveTick`
  (params (DeltaSeconds :type "Float (single-precision)"))
  (bind _cameraboom (`self.CameraBoom`))
  (bind (_returnvalue_x _returnvalue_y) (`KismetMathLibrary.BreakVector` (`SceneComponent.K2_GetComponentLocation` _cameraboom)))
  ; Set camera so it doesn't move on Z axis
  (`SceneComponent.K2_SetWorldLocation` _cameraboom (`KismetMathLibrary.MakeVector` _returnvalue_x _returnvalue_y) false false)
  ; Slowly move camera forward
  (if (not (`self.IsGamePaused`))
    (bind _output_get (set `SpringArmComponent.TargetOffset` (+ (`SpringArmComponent.TargetOffset` _cameraboom) (0.5 0.0 0.0)) _cameraboom))
    ; Die if camera goes too much forward
    (if (> (.x _output_get) (`self.CameraOffsetDeath`))
      (`self.Death`))))

(event `self.Death`
  (bind _returnvalue (`GameplayStatics.GetPlayerController` 0))
  ; Death
  (`KismetSystemLibrary.PrintString` "Ded" true true (struct :`R` 1.0 :`A` 1.0))
  (set `self.IsDead` true)
  (set `self.IsGamePaused` true)
  (bind _returnvalue_2 (`|CreateWidget` "/Game/PERSONAL_CONTENTS/Widgets/WB_Lose.WB_Lose_C" _returnvalue))
  (`UserWidget.AddToViewport` _returnvalue_2 0)
  (set `PlayerController.bShowMouseCursor` true _returnvalue)
  (`WidgetBlueprintLibrary.SetInputMode_UIOnlyEx` _returnvalue _returnvalue_2)
  (`StaticMeshComponent.SetStaticMesh` (`self.DefaultMesh`) "/Game/PERSONAL_CONTENTS/Static_Meshes/Placeholders/Characters/SM_Character_DefaultChicken_Flattened_Placeholder.SM_Character_DefaultChicken_Flattened_Placeholder"))

(fn `RoundMovement`
  (params (Value :type "Float (double-precision)"))
  (returns (NewValue :type "Float (double-precision)"))
  (return (`KismetMathLibrary.Conv_IntToDouble` (* (`KismetMathLibrary.Round` (/ Value 100.0)) 100))))

(fn `UserConstructionScript`)